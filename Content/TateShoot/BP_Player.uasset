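; BP_Player is the player pawn for the TateShoot game, handling movement and rapid fire.
; MoveForward and MoveRight axis inputs add movement along fixed world Y and X axes respectively, independent of the pawn's facing.
; Pressing Shoot fires immediately and starts a fast looping timer that spawns BP_Player_Projectile at the actor's transform until release clears it.
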(event `InputAxis|MoveForward`
  (params (AxisValue :type "Float (single-precision)"))
  (`self.AddMovementInput` (0.0 1.0 0.0) AxisValue))

(event `InputAxis|MoveRight`
  (params (AxisValue :type "Float (single-precision)"))
  (`self.AddMovementInput` (1.0 0.0 0.0) AxisValue))

(event `InputAction|Shoot`
  (params (Key :type "Key Structure"))
  (:`Pressed`
    (bind _returnvalue (`KismetSystemLibrary.K2_SetTimerDelegate` (delegate `ShootLoop`) 0.05 true))
    (set `self.ShootTimer` _returnvalue)
    (`self.ShootLoop`))
  (:`Released`
    (`KismetSystemLibrary.K2_ClearAndInvalidateTimerHandle` (`self.ShootTimer`))))

(event `ShootLoop`
  (`|SpawnActorFromClass` "/Game/TateShoot/BP_Player_Projectile.BP_Player_Projectile_C" (`self.GetTransform`) "Undefined" "OverrideRootScale" null null))

(fn `UserConstructionScript`)